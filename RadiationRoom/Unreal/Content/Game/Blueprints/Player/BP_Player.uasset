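; Player Blueprint for radiation scenarios, handling item interaction, tutorial help and database logging of the user's activity.
; Polls radiation every half second, buffering samples for batched database writes, and logs hand input and timed movement distances.
; Interactions pass through server-to-multicast events, while look-at detection picks the most-hit interactable across several traces.
; An on-demand tutorial buddy swings around to follow camera yaw, and debug keys drive the gameplay manager.
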(event `self.ReceiveBeginPlay`
  (if (`self.IsLocallyControlled`)
    (`|ExecutionSequence`
      (:`then_0`
        (bind _returnvalue (`|GetDataTableRow` "/Game/Game/DataStructures/ControlVars/DT_DefaultVars.DT_DefaultVars" "Data")
          (:`then`
            (bind (_userid _experimentid _grouptype) (break `/Game/Game/DataStructures/ControlVars/F_DefaultVars` _returnvalue))
            (set `self.Name` _userid)
            (set `self.UserType` _grouptype))))
      (:`then_1`
        (`self.BindDataBaseEvents`))
      (:`then_2`
        (bind _asbp_demanded_tutorial_buddy (cast `/Game/Game/Blueprints/Tutorial/BP_DemandedTutorialBuddy` (`ChildActorComponent.ChildActor` (`self.TutorialBuddyComponent`))))
        (set `self.TutorialBuddyActor` _asbp_demanded_tutorial_buddy))
      (:`then_3`
        (`self.MeasureRadiation`)))))

(event `self.ReceiveTick`
  (params (DeltaSeconds :type "Float (single-precision)")))

(event `InitPlayerConditions`)

(event `Key|U`
  (params (Key :type "Key Structure"))
  (:`Pressed`
    (`/Game/Game/Blueprints/Gameplay/BP_GameplayManager.StartScenario` (`/Game/Game/FunctionLibraries/BFL_Common.GetMyGameplayManager`))))

(event `AddDistance`
  (bind _returnvalue (+ (`KismetMathLibrary.Vector_Distance` (`self.Current Position Move VW`) (`SceneComponent.K2_GetComponentLocation` (`self.Mesh`))) (`self.Distance Moved VW`)))
  (if (`self.IsMoving`)
    (if (> _returnvalue 50.0)
      (set `self.Distance Moved VW` _returnvalue)
      (set `self.Current Position Move VW` (`SceneComponent.K2_GetComponentLocation` (`self.Mesh`))))
    (`KismetSystemLibrary.Delay` 0.2)
    (`self.AddDistance`)))

(event `InputAction|DemandHelp`
  (params (Key :type "Key Structure"))
  (bind _tutorialmanager (`/Game/Game/FunctionLibraries/BFL_Common.GetMyTutorialManager`))
  (:`Pressed`
    (`/Engine/EditorBlueprintResources/StandardMacros.IsValid` _tutorialmanager
      (:`Is Valid`
        (`/Game/Game/Blueprints/Tutorial/BP_TutorialManager.DemandedCall` _tutorialmanager)))))

(event `MeasureRadiation`
  (`/Game/Game/Components/AC_Radiation.CalculateRadiation` (`self.AC_Radiation`) (`GameplayStatics.GetWorldDeltaSeconds`))
  (`self.SendUserRadiationEventToDB`)
  (`KismetSystemLibrary.Delay` 0.5)
  (`self.MeasureRadiation`))

(event `/Game/Game/Interfaces/BI_ItemInteract.InteractWith`
  (params (Player :type "/Game/Game/Blueprints/Player/BP_Player Object Reference") (Hand :type "EControllerHand Enum" :default "Left")))

(event `/Game/Game/Interfaces/BI_ItemInteract.CancelInteract`
  (params (Player :type "/Game/Game/Blueprints/Player/BP_Player Object Reference") (Hand :type "EControllerHand Enum" :default "Left")))

(event `Cancel On Server`
  (params (Item :type "/Game/Game/Blueprints/Actors/Items/BP_InteractItemParent Object Reference") (Player :type "/Game/Game/Blueprints/Player/BP_Player Object Reference") (Hand :type "EControllerHand Enum" :default "Left"))
  ;[0.1677 0.1677 0.1677] Interact with
  (`self.Cancel Multi` Item Player Hand))

(event `Interact With On Server`
  (params (`Look At Actor` :type "Actor Object Reference") (Player :type "/Game/Game/Blueprints/Player/BP_Player Object Reference") (Hand :type "EControllerHand Enum" :default "Left"))
  ;[0.1677 0.1677 0.1677] Interact with
  (`/Engine/EditorBlueprintResources/StandardMacros.IsValid` `Look At Actor`
    (:`Is Valid`
      (`self.Interact With Multi` `Look At Actor` Player Hand))))

(event `Interact With Multi`
  (params (`Look At Actor` :type "Actor Object Reference") (Player :type "/Game/Game/Blueprints/Player/BP_Player Object Reference") (Hand :type "EControllerHand Enum" :default "Left"))
  ;[0.1677 0.1677 0.1677] Interact with
  (`/Engine/EditorBlueprintResources/StandardMacros.IsValid` `Look At Actor`
    (:`Is Valid`
      (message `/Game/Game/Interfaces/BI_ItemInteract.InteractWith` `Look At Actor` Player Hand))))

(event `Cancel Multi`
  (params (Item :type "/Game/Game/Blueprints/Actors/Items/BP_InteractItemParent Object Reference") (Player :type "/Game/Game/Blueprints/Player/BP_Player Object Reference") (Hand :type "EControllerHand Enum" :default "Left"))
  ;[0.1677 0.1677 0.1677] Interact with
  (message `/Game/Game/Interfaces/BI_ItemInteract.CancelInteract` Item Player Hand))

(event `BindDataBaseEvents`
  (add `/Game/Game/Components/AC_Database.ED_DatabaseNeedToBeClosed` (`self.AC_Database`) (delegate `OnDatabaseNeedToBeClosed`))
  (add `/Game/Game/Components/AC_Database.ED_DatabaseClosed` (`self.AC_Database`) (delegate `OnDatabaseClosed`)))

(event `OnDatabaseNeedToBeClosed`
  (`self.SendLastEventsToDB`))

(event `OnDatabaseClosed`)

(event `SendUserInputEventToDB`
  (params (input_type :type "InputAction Object Reference") (input_state :type "/Game/Game/DataStructures/Database/E_UserInputState Enum" :default "NewEnumerator0") (hand :type "EControllerHand Enum" :default "Left") (hand_location :type "Vector Structure") (hand_rotation :type "Rotator Structure"))
  (bind _database_manager (`/Game/Game/FunctionLibraries/BFL_Common.GetMyDatabase`))
  (bind _data (`/Game/Game/Blueprints/RR_GameInstance.GetDataBaseMainInfoEvent` (`/Game/Game/FunctionLibraries/BFL_Common.GetMyGameInstance`)))
  (`/Engine/EditorBlueprintResources/StandardMacros.IsValid` _database_manager
    (:`Is Valid`
      (bind (_user_id _experiment_id _scenario_type) (break `/Game/Game/DataStructures/Database/F_MainInfoEvent` _data))
      (`/Game/Game/Blueprints/Database/BP_DataBase_Manager.SendUserInputEventToDB` _database_manager (make `/Game/Game/DataStructures/Database/F_UserInputEvent` 0 _user_id _experiment_id _scenario_type input_type input_state hand hand_location hand_rotation (`KismetMathLibrary.Now`))))))

(event `SendMoveEventToDB`
  (params (move_type :type "/Game/Game/DataStructures/Database/E_MovementType Enum" :default "NewEnumerator0") (start_datetime :type "DateTime Structure") (end_datetime :type "DateTime Structure") (start_position :type "Vector Structure") (end_position :type "Vector Structure") (distance :type "Float (double-precision)"))
  (bind _database_manager (`/Game/Game/FunctionLibraries/BFL_Common.GetMyDataBase`))
  (bind _data (`/Game/Game/Blueprints/RR_GameInstance.GetDataBaseMainInfoEvent` (`/Game/Game/FunctionLibraries/BFL_Common.GetMyGameInstance`)))
  (`/Engine/EditorBlueprintResources/StandardMacros.IsValid` _database_manager
    (:`Is Valid`
      (bind (_user_id _experiment_id _scenario_type) (break `/Game/Game/DataStructures/Database/F_MainInfoEvent` _data))
      (`/Game/Game/Blueprints/Database/BP_DataBase_Manager.Send Move Event to DB` _database_manager (make `/Game/Game/DataStructures/Database/F_MoveEvent` 0 _user_id _experiment_id _scenario_type move_type start_datetime end_datetime start_position end_position distance)))))

(event `SendUserRadiationEventToDB`
  (bind _ac_radiation (`self.AC_Radiation`))
  (bind _returnvalue (`GameplayStatics.GetActorOfClass` "/Game/Game/Blueprints/Actors/Radiation/BP_RadiationEmissionPoint.BP_RadiationEmissionPoint_C"))
  (`/Engine/EditorBlueprintResources/StandardMacros.IsValid` _returnvalue
    (:`Is Valid`
      (`KismetArrayLibrary.Array_Add` (`self.CurrentEventRadiationDoseRateArray`) (`/Game/Game/Components/AC_Radiation.DoseRate` _ac_radiation))
      (`KismetArrayLibrary.Array_Add` (`self.CurrentEventDoseRadiationAbsortionArray`) (`/Game/Game/Components/AC_Radiation.DoseAbsorption` _ac_radiation))
      (`KismetArrayLibrary.Array_Add` (`self.CurrentEventRadiationPositionArray`) (`self.K2_GetActorLocation`))
      (bind _returnvalue_2 (`KismetArrayLibrary.Array_Add` (`self.CurrentEventRadiationDatetimeArray`) (`KismetMathLibrary.Now`)))
      (if (>= _returnvalue_2 9)
        (`self.SendEventsToDB`)))))

(event `SendEventsToDB`
  (`/Game/Game/Components/AC_Database.SendUserRadiationEventToDB` (`self.AC_Database`) :!label _label)
  (`KismetArrayLibrary.Array_Clear` (`self.CurrentEventRadiationDoseRateArray`))
  (`KismetArrayLibrary.Array_Clear` (`self.CurrentEventDoseRadiationAbsortionArray`))
  (`KismetArrayLibrary.Array_Clear` (`self.CurrentEventRadiationPositionArray`))
  (`KismetArrayLibrary.Array_Clear` (`self.CurrentEventRadiationDatetimeArray`)))

(event `SendLastEventsToDB`
  (goto _label))

(event `UserStartMovingInVirtualWorld`
  (if (not (`self.IsMoving`))
    (set `self.IsMoving` true)
    (set `self.Start Datetime Move VW` (`KismetMathLibrary.Now`))
    (bind _output_get (set `self.Start Position Move VW` (`SceneComponent.K2_GetComponentLocation` (`self.Mesh`))))
    (set `self.Current Position Move VW` _output_get)
    (set `self.Distance Moved VW` 0.0)
    (`self.AddDistance`)))

(event `UserStopMovingInVirtualWorld`
  (if (`self.IsMoving`)
    (`|ExecutionSequence`
      (:`then_0`
        (set `self.IsMoving` false)
        (set `self.End Datetime Move VW` (`KismetMathLibrary.Now`))
        (set `self.End Position Move VW` (`SceneComponent.K2_GetComponentLocation` (`self.Mesh`)))
        (set `self.Distance Moved VW` (+ (`KismetMathLibrary.Vector_Distance` (`self.Current Position Move VW`) (`self.End Position Move VW`)) (`self.Distance Moved VW`))))
      (:`then_1`
        (`self.SendMoveEventToDB` "NewEnumerator1" (`self.Start Datetime Move VW`) (`self.End Datetime Move VW`) (`self.Start Position Move VW`) (`self.End Position Move VW`) (/ (`self.Distance Moved VW`) 100.0))))))

(event `AutomaticTuddyOff`
  (set `self.TutorialActive` false :!label _label))

(event `DemandTutorialBuddyHelp`
  (bind _tutorialmanager (`/Game/Game/FunctionLibraries/BFL_Common.GetMyTutorialManager`))
  (bind (_returnvalue_roll _returnvalue_pitch _returnvalue_yaw) (`KismetMathLibrary.BreakRotator` (`SceneComponent.K2_GetComponentRotation` (`self.TuddyPivot`))))
  (bind (_returnvalue_roll_2 _returnvalue_pitch_2 _returnvalue_yaw_2) (`KismetMathLibrary.BreakRotator` (`SceneComponent.K2_GetComponentRotation` (`self.FollowCamera`))))
  (if (`/Game/Game/Components/AC_Cooldown.CooldownCompleted` (`self.AC_Tuddy_Cooldown`))
    (`/Engine/EditorBlueprintResources/StandardMacros.IsValid` _tutorialmanager
      (:`Is Valid`
        (`/Game/Game/Blueprints/Tutorial/BP_TutorialManager.DemandedCall` _tutorialmanager)
        (`/Game/Game/Components/AC_Cooldown.StartCooldown` (`self.AC_Tuddy_Cooldown`))
        (if (`self.TutorialActive`)
          (goto _label)
          (else
            (set `self.TutorialActive` true :!label _label_2)
            (set `self.OldCameraRotation` _returnvalue_yaw_2)
            (set `self.OldTuddyRotation` _returnvalue_yaw)
            (`self.MoveTuddyAroundPlayer`)))))))

(event `AutomaticTuddyOn`
  (goto _label_2))

(event `MoveTuddyAroundPlayer`
  (bind (_returnvalue_roll _returnvalue_pitch _returnvalue_yaw) (`KismetMathLibrary.BreakRotator` (`SceneComponent.K2_GetComponentRotation` (`self.FollowCamera`))))
  (bind (_returnvalue_roll_2 _returnvalue_pitch_2 _returnvalue_yaw_2) (`KismetMathLibrary.BreakRotator` (`SceneComponent.K2_GetComponentRotation` (`self.TuddyPivot`))))
  (if (`self.TutorialActive`)
    (bind (_direction _newtrack_0) (`Timeline|Timeline` :!label _label_3)
      (:`Update`
        (`SceneComponent.K2_SetWorldRotation` (`self.TuddyPivot`) (`KismetMathLibrary.MakeRotator` 0.0 0.0 (`KismetMathLibrary.Lerp` (`self.OldTuddyRotation`) (`self.OldCameraRotation`) _newtrack_0)) false false))
      (:`Finished`
        (if (and (`self.TutorialActive`) (`KismetMathLibrary.InRange_FloatFloat` (- _returnvalue_yaw _returnvalue_yaw_2) -90.0 90.0)) :!label _label_4
          (`KismetSystemLibrary.Delay` 0.1)
          (goto _label_4)
          (else
            (set `self.OldCameraRotation` _returnvalue_yaw)
            (set `self.OldTuddyRotation` _returnvalue_yaw_2)
            (if (`self.TutorialActive`)
              (goto _label_3 :!via `PlayFromStart`))))))))

(event `Key|P`
  (params (Key :type "Key Structure"))
  (:`Pressed`
    (`/Game/Game/Blueprints/Gameplay/BP_GameplayManager.CheatButton` (`/Game/Game/FunctionLibraries/BFL_Common.GetMyGameplayManager`))))

(event `Key|O`
  (params (Key :type "Key Structure"))
  (:`Pressed`
    (if (`/Game/Game/Blueprints/RR_GameInstance.Developing?` (`/Game/Game/FunctionLibraries/BFL_Common.GetMyGameInstance`))
      (`/Game/Game/Blueprints/Gameplay/BP_GameplayManager.LoadNextLevel` (`/Game/Game/FunctionLibraries/BFL_Common.GetMyGameplayManager`)))))

(fn `CheckLookAt`
  (params (Player :type "/Game/Game/Blueprints/Player/BP_Player Object Reference") (`Look from Component` :type "Array of SceneComponent Object Reference") (`Show Laser` :type Boolean :default false))
  (returns (`Look at Actor` :type "Actor Object Reference"))
  (locals (ShowLaser :type "EDrawDebugTrace Enum" :default "ForOneFrame") (HitActors :type "Array of Actor Object Reference") (HitActorsTimes :type "Array of Integer"))
  (bind _hitactorstimes (`local.HitActorsTimes`))
  (for _array_element `Look from Component`
    (bind (_startpoint _endpoint) (`self.LookHitPoint` Player _array_element 250.0))
    (if `Show Laser`
      (set `local.ShowLaser` "ForOneFrame")
      (else
        (set `local.ShowLaser` "None")))
    (bind _outhit (`KismetSystemLibrary.LineTraceSingle` :`Start` _startpoint :`End` _endpoint :`TraceChannel` "TraceTypeQuery2" :`DrawDebugType` (`local.ShowLaser`)))
    (if (or (`KismetSystemLibrary.DoesImplementInterface` (`.HitActor` (`GameplayStatics.BreakHitResult` _outhit)) "/Game/Game/Interfaces/BI_ItemInteract.BI_ItemInteract_C") (`KismetSystemLibrary.DoesImplementInterface` (`.HitActor` (`GameplayStatics.BreakHitResult` _outhit)) "/Game/Game/Interfaces/BI_Use.BI_Use_C"))
      (bind _returnvalue (`KismetArrayLibrary.Array_Find` (`local.HitActors`) (`.HitActor` (`GameplayStatics.BreakHitResult` _outhit))))
      (if (!= _returnvalue -1)
        (`KismetArrayLibrary.Array_Set` _hitactorstimes _returnvalue (+ (`|GetArrayItem` _hitactorstimes _returnvalue) 1))
        (else
          (`KismetArrayLibrary.Array_Add` (`local.HitActors`) (`.HitActor` (`GameplayStatics.BreakHitResult` _outhit)))
          (`KismetArrayLibrary.Array_Add` (`local.HitActorsTimes`))))))
  (if (> (`KismetArrayLibrary.Array_Length` (`local.HitActors`)) 0)
    (return (`|GetArrayItem` (`local.HitActors`) (`KismetMathLibrary.MaxOfIntArray` (`local.HitActorsTimes`))))
    (else
      (return null))))

(fn `GetItemClassFromDataTableByID`
  (params (ItemID :type "/Game/Game/DataStructures/Items/E_ItemType Enum" :default "NewEnumerator2"))
  (returns (`Item Class` :type "Actor Class Reference"))
  (locals (`Current Item Class` :type "Actor Class Reference"))
  (bind _outrownames (`DataTableFunctionLibrary.GetDataTableRowNames` (`self.Items DataTable`)))
  (for _array_element _outrownames
    (bind _returnvalue (`|GetDataTableRow` (`self.Items DataTable`) _array_element)
      (:`then`
        (bind (_grouptype _type _id _name _description _image _mesh _class) (break `/Game/Game/DataStructures/Items/F_ItemData` _returnvalue))
        (if (`|EnumEquality` _type ItemID)
          (set `local.Current Item Class` _class)
          (break)))))
  (return (`local.Current Item Class`)))

(fn `LookHitPoint`
  (params (`From Component` :type "SceneComponent Object Reference") (Distance :type "Float (double-precision)"))
  (returns (StartPoint :type "Vector Structure") (EndPoint :type "Vector Structure"))
  (bind _returnvalue (`SceneComponent.K2_GetComponentLocation` `From Component`))
  (return _returnvalue (+ _returnvalue (* (`KismetMathLibrary.GetForwardVector` (`SceneComponent.K2_GetComponentRotation` `From Component`)) Distance))))

(fn `UserConstructionScript`)