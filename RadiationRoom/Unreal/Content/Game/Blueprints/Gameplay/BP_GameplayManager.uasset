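; Gameplay manager that runs a scenario's data-table quests, tracking current, active and completed quests and registering itself on the GameInstance.
; Quest changes notify an event dispatcher; completions update quest list and scenario description widgets, then recheck overall completion.
; Quest states and start/finish markers go to the database, and ending gameplay loads the next level or quits.
; Player, item, place-point, NPC and Tuddy binding events are empty stubs; a cheat event skips quests.
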(event `CheatButton`
  ;[1 1 1] Cheat Button
  (`self.CompleteQuest` (`|GetArrayItem` (`self.SortedQuests`) (`self.CurrentQuestIndex`)))
  (if (< (`self.CurrentQuestIndex`) (- (`KismetArrayLibrary.Array_Length` (`self.SortedQuests`)) 1))
    (bind _result (`/Engine/EditorBlueprintResources/StandardMacros.IncrementInt` (`self.CurrentQuestIndex`))
      (:`  `
        (`self.SetCurrentQuest` (`|GetArrayItem` (`self.SortedQuests`) _result))))))

(event `self.ReceiveBeginPlay`
  (`|ExecutionSequence`
    (:`then_0`
      (`self.BindGameInstanceActions`)
      (`self.BindItemActions`)
      (`self.BindPlacePointsActions`)
      (`self.BindNPCActions`)
      (`self.BindTuddyActions`)
      (`self.BindPlayerActions`))
    (:`then_1`
      (set `/Game/Game/Blueprints/RR_GameInstance.GameplayManager` self (`/Game/Game/FunctionLibraries/BFL_Common.GetMyGameInstance`))
      (`/Game/Game/Blueprints/Tutorial/BP_TutorialManager.OnGameInstanceDefaultVarsSetted` (`self.TutorialManager`))
      (bind _outactors (`GameplayStatics.GetAllActorsOfClass` "/Game/Game/Blueprints/Widgets/QuestPanels/BP_QuestList.BP_QuestList_C"))
      (set `self.QuestListWidget` _outactors))
    (:`then_2`
      (set `self.GameplayCompleted` false)
      (if (`self.QuestAreSorted`)
        (`self.ED_OrderedGameplay`)))
    (:`then_3`
      (bind _outrownames (`DataTableFunctionLibrary.GetDataTableRowNames` (`self.Quest Data Table`)))
      (for _array_element _outrownames
        (`BlueprintMapLibrary.Map_Add` (`self.CompletedQuests`) _array_element)
        (`KismetArrayLibrary.Array_AddUnique` (`self.SortedQuests`) _array_element)))))

(event `ActivateQuests`
  (params (QuestIDsList :type "Array of Name"))
  (for _array_element QuestIDsList
    (`self.AddActiveQuest` _array_element)))

(event `SetCurrentQuest`
  (params (`Quest ID` :type Name))
  (bind _output_get (set `self.CurrentQuestID` `Quest ID`))
  (`self.AddActiveQuest` _output_get)
  (bind _quest_data (`self.Get Quest Data By ID` (`self.CurrentQuestID`)))
  (set `self.CurrentQuestData` _quest_data)
  (`self.ED_QuestChanged` (`self.CurrentQuestID`))
  (`self.Send Quest to Database` (`self.CurrentQuestID`) "NewEnumerator1"))

(event `CompleteQuest`
  (params (QuestID :type Name))
  (`|ExecutionSequence`
    (:`then_0`
      (`self.Send Quest to Database` QuestID "NewEnumerator3")
      (`BlueprintMapLibrary.Map_Add` (`self.CompletedQuests`) QuestID true)
      (`self.RemoveActiveQuest` QuestID))
    (:`then_1`
      (for _array_element (`self.QuestListWidget`)
        (`/Game/Game/Blueprints/Widgets/QuestPanels/BP_QuestList.CompleteQuest` _array_element QuestID)))
    (:`then_2`
      (bind _returnvalue (`GameplayStatics.GetActorOfClass` "/Game/Game/Blueprints/Widgets/QuestPanels/BP_ScenarioDescriptionActor.BP_ScenarioDescriptionActor_C"))
      (`/Engine/EditorBlueprintResources/StandardMacros.IsValid` _returnvalue
        (:`Is Valid`
          (bind _descriptionwidget (`/Game/Game/Blueprints/Widgets/QuestPanels/BP_ScenarioDescriptionActor.DescriptionWidget` _returnvalue)
            (:`then`
              (`/Game/Game/UserInterfaces/QuestPanels/WBP_ScenarioDescription.CompleteTask` _descriptionwidget QuestID))
            (:`else`)))))
    (:`then_3`
      (`self.Is Gameplay Completed`))))

(event `EndGameplay`
  (`self.SendFinishEventToDB`)
  (`/Game/Game/Blueprints/RR_GameInstance.SetGameplayStepsData` (`/Game/Game/FunctionLibraries/BFL_Common.GetMyGameInstance`) (`self.QuestsList`))
  (`KismetSystemLibrary.Delay` 0.5)
  (`self.LoadNextLevel`))

(event `BindGameInstanceActions`
  (add `/Game/Game/Blueprints/RR_GameInstance.ED_DatabaseClosed` (`/Game/Game/FunctionLibraries/BFL_Common.GetMyGameInstance`) (delegate `OnDatabaseClosed`))
  (add `/Game/Game/Blueprints/RR_GameInstance.ED_PlayerSetted` (`/Game/Game/FunctionLibraries/BFL_Common.GetMyGameInstance`) (delegate `OnGameInstancePlayerSetted`)))

(event `OnDatabaseClosed`)

(event `OnGameInstancePlayerSetted`
  (`self.BindPlayerActions`))

(event `LoadNextLevel`
  (bind (_exit _next_scenario_data) (`/Game/Game/FunctionLibraries/BFL_Scenarios.GetCurrentScenarioNextData`))
  (if _exit
    (`KismetSystemLibrary.Delay` 0.5)
    (`KismetSystemLibrary.QuitGame` null "Quit")
    (else
      (bind _output_get (set `/Game/Game/Blueprints/RR_GameInstance.Level to Load` (`.BPLevelName_28_4768376E42D10726E2307A90E7F79D29` (break `/Game/Game/DataStructures/Scenarios/F_ScenarioData` _next_scenario_data)) (`/Game/Game/FunctionLibraries/BFL_Common.GetMyGameInstance`)))
      (`GameplayStatics.OpenLevel` _output_get))))

(event `StartScenario`
  (`self.SendStartEventToDB`))

(event `SendStartEventToDB`
  (`self.Send Quest to Database` "00001" "NewEnumerator3"))

(event `AddItemToGameManagerImportantList`
  (params (ItemType :type "/Game/Game/DataStructures/Items/E_ItemType Enum" :default "NewEnumerator2") (Actor :type "Actor Object Reference")))

(event `SendFinishEventToDB`
  (`self.Send Quest to Database` "00002" "NewEnumerator3"))

(event `BindPlayerActions`)

(event `BindItemActions`)

(event `BindPlacePointsActions`)

(event `BindNPCActions`)

(event `BindTuddyActions`)

(fn `AddActiveQuest`
  (params (`Quest ID` :type Name))
  (`KismetArrayLibrary.Array_AddUnique` (`self.ActiveQuests`) `Quest ID`))

(fn `Get Quest Data By ID`
  (params (`Quest ID` :type Name))
  (returns (`Quest Data` :type "/Game/Game/DataStructures/Gameplay/F_GameplayStepData Structure"))
  (bind _returnvalue (`|GetDataTableRow` (`self.Quest Data Table`) `Quest ID`)
    (:`then`
      (return _returnvalue))
    (:`RowNotFound`
      (`/Game/Game/Blueprints/RR_GameInstance.Log` (`/Game/Game/FunctionLibraries/BFL_Common.GetMyGameInstance`) "NewEnumerator2" (`|FormatText` "La quest {row_name} no existe en la tabla" `Quest ID`) false)
      (return))))

(fn `Is Current Quest`
  (params (QuestID :type Name))
  (returns (Yes :type Boolean))
  (return (== QuestID (`self.CurrentQuestID`))))

(fn `Is Current Quest and Can Start`
  (params (QuestID :type Name))
  (returns (`Yes / No` :type Boolean))
  (return (and (`self.Is Current Quest` QuestID) (`self.CanStartCurrentQuest`))))

(fn `Is Gameplay Completed`
  (bind _values (`BlueprintMapLibrary.Map_Values` (`self.CompletedQuests`)))
  (for _array_element _values
    (if _array_element
      (set `self.GameplayCompleted` true)
      (else
        (set `self.GameplayCompleted` false)
        (break)))))

(fn `IsQuestCompleted`
  (params (`Quest ID` :type Name))
  (returns (`Quest Completed` :type Boolean))
  (return (`BlueprintMapLibrary.Map_Find` (`self.CompletedQuests`) `Quest ID`)))

(fn `RemoveActiveQuest`
  (params (QuestID :type "Name (by ref)"))
  (`KismetArrayLibrary.Array_RemoveItem` (`self.ActiveQuests`) QuestID))

(fn `Send Quest to Database`
  (params (`Quest ID` :type Name) (`Step State` :type "/Game/Game/DataStructures/Gameplay/E_GameplayStepState Enum" :default "NewEnumerator0"))
  (bind _database_manager (`/Game/Game/FunctionLibraries/BFL_Common.GetMyDataBase`))
  (bind _data (`/Game/Game/Blueprints/RR_GameInstance.GetDataBaseMainInfoEvent` (`/Game/Game/FunctionLibraries/BFL_Common.GetMyGameInstance`)))
  (`/Engine/EditorBlueprintResources/StandardMacros.IsValid` _database_manager
    (:`Is Valid`
      (bind (_user_id _experiment_id _scenario_type) (break `/Game/Game/DataStructures/Database/F_MainInfoEvent` _data))
      (`/Game/Game/Blueprints/Database/BP_DataBase_Manager.Send Gameplay Event to DB` _database_manager (make `/Game/Game/DataStructures/Database/F_GameplayEvent` 0 _user_id _experiment_id _scenario_type `Quest ID` `Step State` (`KismetMathLibrary.Now`))))))

(fn `UserConstructionScript`)