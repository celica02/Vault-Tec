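; Actor component for BP_NPC_Talkable that runs NPC conversations with the player.
; On BeginPlay it caches the dialog widget and loads conversations from a DataTable.
; Each line waits its delay, then shows as player or NPC text in WBP_Dialog, with typewriter completion advancing to the next.
; Conversation start and stop are logged to the database; per-line voice playback exists but is disconnected.
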(event `self.ReceiveBeginPlay`
  (`|ExecutionSequence`
    (:`then_0`
      (bind _asbp_npc_talkable (cast `/Game/Game/Blueprints/Characters/BP_NPC_Talkable` (`self.GetOwner`)))
      (set `self.Owner` _asbp_npc_talkable))
    (:`then_1`
      (bind _dialogwidgetcomponent (`/Game/Game/Blueprints/Characters/BP_NPC_Talkable.DialogWidgetComponent` (`self.Owner`))
        (:`then`
          (`SceneComponent.SetHiddenInGame` _dialogwidgetcomponent false false)
          (bind _aswbp_dialog (cast `/Game/Game/UserInterfaces/Dialogs/WBP_Dialog` (`WidgetComponent.GetWidget` _dialogwidgetcomponent)))
          (bind _output_get (set `self.Widget` _aswbp_dialog))
          (`/Game/Game/UserInterfaces/Dialogs/WBP_Dialog.SetOwner` _output_get (`self.Owner`)))
        (:`else`)))
    (:`then_2`
      (`self.SetDialogsFromDataTable`))))

(event `self.ReceiveTick`
  (params (DeltaSeconds :type "Float (single-precision)")))

(event `SetTypewriterComponent`
  (params (TypewriterComponent :type "TypewriterTextComponent Object Reference"))
  (bind _output_get (set `self.TypewriterComponent` TypewriterComponent))
  (bind _output_get_2 (set `/Game/Game/UserInterfaces/Dialogs/WBP_Dialog.TypewriterComponent` _output_get (`self.Widget`)))
  (add `TypewriterTextComponent.OnCompleted` _output_get_2 (delegate `OnTypewriterFinished`)))

(event `Interact With`
  ;[1 1 1] Interact with
  (if (not (`self.IsTalking?`))
    (`self.StartConversation`)
    (`self.SendDialogEventToDB` "NewEnumerator10")
    (`/Game/Game/Blueprints/Characters/BP_NPC_Talkable.ED_ConversationStarted` (`self.Owner`))))

(event `StartConversation`
  ;[1 1 1] Conversation
  (bind _isempty (`self.Is Conversation Empty`))
  (if (and (not _isempty) (`self.CanStartConversation?`))
    (set `self.IsTalking?` true)
    (`AudioComponent.Play` (`/Game/Game/Blueprints/Characters/BP_NPC.Audio` (`self.Owner`)) 0.0)
    (set `self.DialogIndex` 0)
    (`self.ProcessDialog`)
    (if (`self.ShowDialogPanel`)
      (`SceneComponent.SetHiddenInGame` (`/Game/Game/Blueprints/Characters/BP_NPC_Talkable.DialogWidgetComponent` (`self.Owner`)) false false)
      (`/Game/Game/UserInterfaces/Dialogs/WBP_Dialog.ShowDialogBox` (`self.Widget`)))))

(event `StopConversation`
  ;[1 1 1] Conversation
  (if (`self.IsTalking?`)
    (set `self.IsTalking?` false)
    (`AudioComponent.Stop` (`/Game/Game/Blueprints/Characters/BP_NPC.Audio` (`self.Owner`)))
    (`self.SendDialogEventToDB` "NewEnumerator28")
    (`self.ConversationFinished` (`self.ConversationIndex`))
    (if (`self.ShowDialogPanel`)
      (`SceneComponent.SetHiddenInGame` (`/Game/Game/Blueprints/Characters/BP_NPC_Talkable.DialogWidgetComponent` (`self.Owner`)) true false)
      (`/Game/Game/UserInterfaces/Dialogs/WBP_Dialog.HideDialogBox` (`self.Widget`)))))

(event `ContinueDialog`
  ;[1 1 1] Process Dialog
  (`self.ProcessDialog`))

(event `ProcessDialog`
  ;[1 1 1] Process Dialog
  (if (`self.IsTalking?`)
    (bind _dialog (`self.GetCurrentDialog`))
    (bind (_type _text _voice _timetoplay) (break `/Game/Game/DataStructures/Dialogs/F_DialogLine` _dialog))
    (`KismetSystemLibrary.Delay` _timetoplay)
    (switch `/Game/Game/DataStructures/Dialogs/E_DialogType` _type
      (:`NewEnumerator2`
        (`KismetSystemLibrary.PrintString` "Un diálogo que no tiene dueño :(" true true (struct :`R` 1.0 :`A` 1.0)))
      (:`NewEnumerator0`
        (`self.CreatePlayerDialog`))
      (:`NewEnumerator1`
        (`self.CreateNPCDialog`)))))

(event `OnTypewriterFinished`
  (`KismetSystemLibrary.Delay` 1.0)
  (if (`self.IsTalking?`)
    (bind _continue (`self.Next Dialog`))
    (if _continue
      (`self.ProcessDialog`)
      (else
        (`self.StopConversation`)))))

(event `PlayDialogSound`
  (bind _audio (`/Game/Game/Blueprints/Characters/BP_NPC.Audio` (`self.Owner`)))
  ;[1 1 1] Sound
  (bind _dialog (`self.GetCurrentDialog`))
  (`AudioComponent.SetSound` _audio (`.Voice_6_2E5887994B1F4CDC62FF08989CA7335B` (break `/Game/Game/DataStructures/Dialogs/F_DialogLine` _dialog)))
  (`AudioComponent.Play` _audio 0.0)
  (add `AudioComponent.OnAudioFinished` _audio (delegate `OnDialogSoundFinished`)))

(event `OnDialogSoundFinished`
  ;[1 1 1] Sound
  (if (and (`self.IsTalking?`) (not false))
    (`KismetSystemLibrary.Delay` 0.2)
    (bind _continue (`self.Next Dialog`))
    (if _continue
      (`self.ProcessDialog`)
      (else
        (`self.StopConversation`)))))

(event `SendDialogEventToDB`
  (params (`Event Type` :type "/Game/Game/DataStructures/Database/E_NPCEventType Enum" :default "NewEnumerator5") (hand :type "EControllerHand Enum" :default "Left"))
  ;[1 1 1] Database
  (bind _data (`/Game/Game/Blueprints/RR_GameInstance.GetDataBaseMainInfoEvent` (`/Game/Game/Blueprints/Characters/BP_NPC.GameInstance` (`self.Owner`))))
  (bind (_user_id _experiment_id _scenario_type) (break `/Game/Game/DataStructures/Database/F_MainInfoEvent` _data))
  (`/Game/Game/Blueprints/Database/BP_DataBase_Manager.Send NPC Interaction Event to DB` (`/Game/Game/Blueprints/RR_GameInstance.Database Manager` (`/Game/Game/Blueprints/Characters/BP_NPC.GameInstance` (`self.Owner`))) (make `/Game/Game/DataStructures/Database/F_NPCInteractionEvent` 0 _user_id _experiment_id _scenario_type (`/Game/Game/Blueprints/Characters/BP_NPC.ActorId` (`self.Owner`)) (`self.ConversationIndex`) `Event Type` hand (`KismetMathLibrary.Now`))))

(fn `CreateNPCDialog`
  (if (`self.ShowDialogPanel`)
    (bind _dialog (`self.GetCurrentDialog`))
    (`/Game/Game/UserInterfaces/Dialogs/WBP_Dialog.CreateNPCText` (`self.Widget`) (`KismetTextLibrary.Conv_StringToText` (`/Game/Game/Blueprints/Characters/BP_NPC.Name` (`self.Owner`))) (`.Text_2_8889C3EB4A46B35524B709947C974DCC` (break `/Game/Game/DataStructures/Dialogs/F_DialogLine` _dialog)))))

(fn `CreatePlayerDialog`
  (if (`self.ShowDialogPanel`)
    (bind _dialog (`self.GetCurrentDialog`))
    (`/Game/Game/UserInterfaces/Dialogs/WBP_Dialog.CreatePlayerText` (`self.Widget`) (`KismetTextLibrary.Conv_StringToText` (`/Game/Game/Blueprints/Player/BP_Player.Name` (`/Game/Game/FunctionLibraries/BFL_Common.GetMyPlayer`))) (`.Text_2_8889C3EB4A46B35524B709947C974DCC` (break `/Game/Game/DataStructures/Dialogs/F_DialogLine` _dialog)))))

(fn `GetCurrentConversation`
  (returns (CurrentConversation :type "/Game/Game/DataStructures/Dialogs/F_Conversation Structure (by ref)"))
  (return (`|GetArrayItem` (`self.Conversations`) (`self.ConversationIndex`))))

(fn `GetCurrentDialog`
  (returns (Dialog :type "/Game/Game/DataStructures/Dialogs/F_DialogLine Structure"))
  (return (`|GetArrayItem` (`.DialogData_39_CA31413047BF35DEDAF362AFEAA84133` (break `/Game/Game/DataStructures/Dialogs/F_Conversation` (`|GetArrayItem` (`self.Conversations`) (`self.ConversationIndex`)))) (`self.DialogIndex`))))

(fn `GetNumberOfConversations`
  (params (`List of Dialogs` :type "Array of String"))
  (returns (`Number of Conversations` :type Integer))
  (locals (AuxSet :type "Set of String"))
  (for _array_element `List of Dialogs`
    (`BlueprintSetLibrary.Set_Add` (`local.AuxSet`) _array_element))
  (return (`BlueprintSetLibrary.Set_Length` (`local.AuxSet`))))

(fn `Is Conversation Empty`
  (returns (IsEmpty :type Boolean))
  (return (== (`KismetArrayLibrary.Array_Length` (`self.Conversations`)) 0)))

(fn `Next Dialog`
  (returns (Continue :type Boolean))
  (bind _returnvalue (`KismetArrayLibrary.Array_Length` (`.DialogData_39_CA31413047BF35DEDAF362AFEAA84133` (break `/Game/Game/DataStructures/Dialogs/F_Conversation` (`|GetArrayItem` (`self.Conversations`) (`self.ConversationIndex`))))))
  (if (and (> _returnvalue 0) (< (+ (`self.DialogIndex`) 1) _returnvalue))
    (`/Engine/EditorBlueprintResources/StandardMacros.IncrementInt` (`self.DialogIndex`)
      (:`  `
        (return true)))
    (else
      (return false))))

(fn `NextConversation`
  (bind _isempty (`self.Is Conversation Empty`))
  (if (and (not _isempty) (< (`self.ConversationIndex`) (- (`KismetArrayLibrary.Array_Length` (`self.Conversations`)) 1)))
    (set `self.ConversationIndex` (+ (`self.ConversationIndex`) 1))))

(fn `SetDialogsFromDataTable`
  (`KismetArrayLibrary.Array_Clear` (`self.Conversations`))
  (bind _dialog_data_table (`self.Dialog Data Table`)
    (:`then`
      (bind _outrownames (`DataTableFunctionLibrary.GetDataTableRowNames` _dialog_data_table))
      (for _array_element _outrownames
        (bind _returnvalue (`|GetDataTableRow` _dialog_data_table _array_element)
          (:`then`
            (bind (_conversationnumber _dialogdata) (break `/Game/Game/DataStructures/Dialogs/F_Conversation` _returnvalue))
            (`KismetArrayLibrary.Array_Add` (`self.Conversations`) (make `/Game/Game/DataStructures/Dialogs/F_Conversation` _conversationnumber _dialogdata))))))
    (:`else`)))